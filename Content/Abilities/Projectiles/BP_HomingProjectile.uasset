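; Homing projectile Blueprint for MOBA targets that flies at one selectable target and ignores overlaps with anything else.
; HomeToTarget stores the target and adds a static mesh component to it as the movement component's homing target.
; Mesh overlap with that target destroys the projectile, and the Destroyed event calls the hit dispatcher, whatever the cause of destruction.
; Setters store owning actor and ability; the BasicAttack hit gameplay-event logic is disconnected.
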(event `self.ReceiveBeginPlay`
  (`parent.ReceiveBeginPlay`))

(event `self.ReceiveActorBeginOverlap`
  (params (OtherActor :type "Actor Object Reference")))

(event `self.ProjectileMesh.OnComponentBeginOverlap`
  (params (OverlappedComponent :type "PrimitiveComponent Object Reference") (OtherActor :type "Actor Object Reference") (OtherComp :type "PrimitiveComponent Object Reference") (OtherBodyIndex :type Integer) (bFromSweep :type Boolean) (SweepResult :type "HitResult Structure (by ref)"))
  (bind _projectile_target (`self.Projectile Target`))
  (bind _asmoba_selectable (cast `MobaSelectable` OtherActor))
  (if (`KismetSystemLibrary.IsValid` _projectile_target)
    (if (== _asmoba_selectable _projectile_target)
      (`self.K2_DestroyActor`))))

(event `self.ReceiveDestroyed`
  (`self.ProjectileHitDispatcher`))

(fn `Home To Target`
  (params (`Projectile Target` :type "MobaSelectable Object Reference"))
  (bind _output_get (set `self.Projectile Target` `Projectile Target`))
  (bind _returnvalue (`AddComponent|NODE_AddStaticMeshComponent-0` :`self` _output_get))
  (if (`KismetSystemLibrary.IsValid` _returnvalue)
    (set `ProjectileMovementComponent.HomingTargetComponent` _returnvalue (`self.ProjectileMovement`))))

(fn `Set Owner`
  (params (NewOwner :type "MobaSelectable Object Reference"))
  (set `self.OwningActor` NewOwner))

(fn `Set Owning Ability`
  (params (`New Owning Ability` :type "/Game/Abilities/BasicAttack/GA_ProjectileBasicAttack Object Reference"))
  (set `self.Owning Ability` `New Owning Ability`))

(fn `UserConstructionScript`
  (`parent.UserConstructionScript`))